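; First-person player character that handles crouch input, proximity-style voice chat and positioning of held objects.
; A second after BeginPlay, it creates a VOIP talker from a valid PlayerState, attached to the capsule with voice attenuation.
; The locally controlled player also toggles speaking and enables voice loopback through console commands.
; SetGrabLocation moves a given handle's target to grab distance ahead of the camera along control rotation, shifted sideways by an offset.
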(event `self.ReceiveBeginPlay`
  (`KismetSystemLibrary.Delay` 1.0)
  (`self.InitializeVoiceChat`))

(event `self.ReceiveTick`
  (params (DeltaSeconds :type "Float (single-precision)")))

(event `EnhancedInput|/Game/DownDog/Input/Actions/IA_Crouch`
  (params (ActionValue :type "Vector2D Structure") (ElapsedSeconds :type "Float (double-precision)") (TriggeredSeconds :type "Float (double-precision)") (InputAction :type "InputAction Object Reference" :default "/Game/DownDog/Input/Actions/IA_Crouch.IA_Crouch"))
  (:`Started`
    (`self.Crouch`))
  (:`Completed`
    (`self.UnCrouch`)))

(event `InitializeVoiceChat`
  (bind _playerstate (`self.PlayerState`)
    (:`then`
      (bind _returnvalue (`VOIPTalker.CreateTalkerForPlayer` _playerstate))
      (set `self.VOIP` _returnvalue)
      (`VOIPStatics.SetMicThreshold` -1.0)
      (set `VOIPTalker.Settings` (make `VoiceSettings` (`self.CapsuleComponent`) "/Game/DownDog/Core/Character/ATT_CharacterVoice.ATT_CharacterVoice") (`self.VOIP`))
      (if (`self.IsLocallyControlled`)
        (`KismetSystemLibrary.ExecuteConsoleCommand` "OSS.VoiceLoopback 1" null)
        (`KismetSystemLibrary.ExecuteConsoleCommand` "ToggleSpeaking 1" null)))
    (:`else`)))

(fn `SetGrabLocation`
  (params (Handle :type "PhysicsHandleComponent Object Reference") (GrabOffset :type "Float (double-precision)"))
  (bind _returnvalue (`Controller.GetControlRotation` (`self.GetController`)))
  (`PhysicsHandleComponent.SetTargetLocation` (`local.Handle`) (+ (`SceneComponent.K2_GetComponentLocation` (`self.FirstPersonCameraComponent`)) (* (`KismetMathLibrary.GetForwardVector` _returnvalue) (`self.GrabDistance`)) (* (`KismetMathLibrary.GetRightVector` _returnvalue) (`local.GrabOffset`)))))

(fn `UserConstructionScript`)