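; BP_DropItem is a menu actor that spawns household props, such as ceramics, a fridge and a couch, around its location.
; BeginPlay starts a looping timer, presumably bound to DropItem, the only custom event.
; DropItem spawns the next class from a fixed, ceramic-heavy sequence with random horizontal offset and rotation, then advances the index and wraps to the start.
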(event `self.ReceiveBeginPlay`
  (`KismetSystemLibrary.K2_SetTimerDelegate` (`|CreateDelegate` :!event `DropItem`) 4.0 true))

(event `DropItem`
  (bind _returnvalue (`KismetMathLibrary.RandomFloatInRange` -50.0 50.0))
  (bind _array (`|MakeArray` "/Game/DownDog/Items/BP_Ceramic.BP_Ceramic_C" "/Game/DownDog/Items/BP_Ceramic.BP_Ceramic_C" "/Game/DownDog/Items/Fridge/BP_Fridge.BP_Fridge_C" "/Game/DownDog/Items/BP_Ceramic.BP_Ceramic_C" "/Game/DownDog/Items/BP_Ceramic.BP_Ceramic_C" "/Game/DownDog/Items/Couch/BP_Couch.BP_Couch_C" "/Game/DownDog/Items/BP_Ceramic.BP_Ceramic_C" :!type "Actor Class Reference"))
  (`|SpawnActorFromClass` (`|GetArrayItem` _array (`self.Item`)) (`KismetMathLibrary.MakeTransform` (+ (`self.K2_GetActorLocation`) (`KismetMathLibrary.MakeVector` _returnvalue _returnvalue)) (`KismetMathLibrary.RandomRotator` true)) "Undefined" "MultiplyWithRoot" null null)
  (`/Engine/EditorBlueprintResources/StandardMacros.IncrementInt` (`self.Item`)
    (:`  `
      (if (>= (`self.Item`) (`KismetArrayLibrary.Array_Length` _array))
        (set `self.Item` 0)))))

(fn `UserConstructionScript`)